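; BP_Performance is an effects actor for a sound performance, firing particle bursts whenever its Beat event is called.
; Beat flips a boolean to alternate between scaled-up sparks with an explosion and scaled-up smoke.
; It also increments a beat counter and prints its value modulo 4 as a repeating four-count readout.
; BeginPlay, overlap, Tick and the construction script are empty, so Beat must be triggered externally.
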(event Custom|Beat
  (bind _p_smoke (Variables|Default|GetP_Smoke))
  (bind _beatcount (Variables|Default|GetBeatCount))
  (bind _p_sparks (Variables|Default|GetP_Sparks))
  (Utilities|FlowControl|Sequence
    (:then_0
      (if (Variables|Default|GetCondition)
        (Components|Activation|Activate _p_sparks true)
        (Transformation|SetWorldScale3D _p_sparks "3.000000,3.000000,3.000000")
        (Variables|Default|SetCondition false)
        (else
          (Components|Activation|Activate _p_smoke true)
          (Transformation|SetWorldScale3D _p_smoke "5.000000,5.000000,5.000000")
          (Variables|Default|SetCondition true))))
    (:then_1
      (Development|PrintString (Utilities|String|ToString(Integer) (Math|Integer|%(Integer) _beatcount 4)))
      (Math|Integer|IncrementInt _beatcount))))

(event EventBeginPlay)

(event Collision|EventActorBeginOverlap
  (params (OtherActor :type Actor%20Object%20Reference)))

(event EventTick
  (params (DeltaSeconds :type Float%20%28single-precision%29)))

(fn ConstructionScript)